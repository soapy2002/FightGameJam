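; Shared camera actor that frames two players, following their midpoint along Y and Z.
; Shortly after BeginPlay it takes the first two BP_BasePlayer actors found and enables tracking.
; Each Tick, CameraAdjust moves the actor and Sphere to the midpoint, raised vertically, taking actor X from the camera.
; Spring arm length zooms with the signed Y gap (Player2 minus Player1), clamped to a range, with debug prints.
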(event EventBeginPlay
  (Utilities|FlowControl|Delay 0.2)
  (bind _outactors (Actor|GetAllActorsOfClass "/Game/BP/CharacterBP/BP_BasePlayer.BP_BasePlayer_C"))
  (bind _output_get (Variables|Default|SetPlayer1 (Utilities|Array|Get(acopy) _outactors)))
  (bind _output_get_2 (Variables|Default|SetPlayer2 (Utilities|Array|Get(acopy) _outactors 1)))
  (Development|PrintString (Utilities|String|Append "Player 1: " (Utilities|GetDisplayName _output_get) "Player 2: " (Utilities|GetDisplayName _output_get_2)))
  (Variables|Default|SetPlayer's%20Alive? true))

(event EventTick
  (params (DeltaSeconds :type Float%20%28single-precision%29))
  (CallFunction|CameraAdjust)
  (Development|PrintString (Utilities|String|ToString(Float) (Variables|/Script/Engine.SpringArmComponent|GetTargetArmLength (Variables|Default|GetSpringArm)))))

(fn ConstructionScript)

(fn CameraAdjust
  (bind _player1 (Variables|Default|GetPlayer1))
  (bind _player2 (Variables|Default|GetPlayer2))
  (bind _capsulecomponent (Variables|/Script/Engine.Character|GetCapsuleComponent _player2))
  (bind _capsulecomponent_2 (Variables|/Script/Engine.Character|GetCapsuleComponent _player1))
  (bind _returnvalue (Transformation|GetWorldLocation _capsulecomponent))
  (bind _returnvalue_2 (Transformation|GetWorldLocation _capsulecomponent_2))
  (bind _returnvalue_3 (- (.y _returnvalue) (.y _returnvalue_2)))
  (bind _returnvalue_4 (+ (.z _returnvalue_2) (.z _returnvalue)))
  (bind _returnvalue_5 (/ _returnvalue_4 2.0))
  (bind _returnvalue_6 (+ _returnvalue_5 3e+02))
  (if (Variables|Default|GetPlayer's%20Alive?)
    (bind _output_get (Variables|Default|SetPlayerDistance (+ (.y _returnvalue_2) (.y _returnvalue))))
    ;[0.15 0.15 0.15 0.5] Comment
    (bind _output_get_2 (Variables|Default|SetPlayer%20Midpoint (/ _output_get 2.0)))
    (Transformation|SetActorLocation (Math|Vector|MakeVector (.x (Transformation|GetWorldLocation (Variables|Default|GetCamera))) _output_get_2 _returnvalue_6) false false)
    (Variables|Default|SetPlayer%20Height%20Midpoint _returnvalue_5)
    (Transformation|SetWorldLocation (Variables|Default|GetSphere) (Math|Vector|MakeVector 0.0 (/ _output_get 2.0) _returnvalue_6) false false)
    (Development|PrintString (Utilities|String|ToString(Float) _returnvalue_3))
    (Variables|/Script/Engine.SpringArmComponent|SetTargetArmLength (Variables|Default|GetSpringArm) (Math|Float|Clamp(Float) _returnvalue_3 9.5e+02 1.6e+03))))