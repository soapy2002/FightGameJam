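; Base player character for a two-player fighting game, with two stances that each have their own health pool.
; Current stance selects punch or kick montages and block (with perfect-block window) or dash, while a decaying timer and counter track combos.
; Depleting a stance passes overflow damage to the other and destroys cable components.
; It also updates the shared HUD by player index, toggles pause and reports round events to the GameInstance.
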(event Custom|StanceFailed
  ;[0.15 0.15 0.15 0.5] Stance Changing
)

(event Custom|HaltMovement
  ;[0.15 0.15 0.15 0.5] Basic Actions
  (Variables|/Script/Engine.CharacterMovementComponent|SetMaxWalkSpeed (Variables|Character|GetCharacterMovement) 0.0))

(event Custom|IncreaseComboTimer
  ;[0.15 0.15 0.15 0.5] Combo Managment
  (Variables|Default|SetComboTimer (+ (Variables|Default|GetComboTimer) 2.0)))

(event Custom|LightAttack_Punch
  ;[0.15 0.15 0.15 0.5] Punching and Kicking
  (if (<= (Variables|Default|GetComboChecker) 1)
    (Math|Integer|IncrementInt (Variables|Default|GetComboChecker)
      (:%20%20
        (CallFunction|IncreaseComboTimer)))
    (else
      (Variables|Default|SetComboChecker 0)
      (Variables|Default|SetJabbing true)))
  (Utilities|FlowControl|FlipFlop
    (:A
      (bind _returnvalue (Animation|PlayAnimMontage "/Game/BP/CharacterBP/Anim/AM_Attack_Right_Montage.AM_Attack_Right_Montage" 1.0 "None"))
      (CallFunction|HaltMovement)
      (CallFunction|ComboUpdater)
      (Utilities|FlowControl|Delay _returnvalue)
      (CallFunction|UnlockAttack))
    (:B
      (bind _returnvalue_2 (Animation|PlayAnimMontage "/Game/BP/CharacterBP/Anim/AM_Attack_Left_Montage.AM_Attack_Left_Montage" 1.0 "None"))
      (CallFunction|HaltMovement)
      (CallFunction|ComboUpdater)
      (Utilities|FlowControl|Delay _returnvalue_2)
      (CallFunction|UnlockAttack))))

(event Custom|LightAttack_Kick
  ;[0.15 0.15 0.15 0.5] Punching and Kicking
  (if (<= (Variables|Default|GetComboChecker) 1)
    (Math|Integer|IncrementInt (Variables|Default|GetComboChecker)
      (:%20%20
        (CallFunction|IncreaseComboTimer)))
    (else
      (Variables|Default|SetComboChecker 0)))
  (Variables|Default|SetIsLightKicking? true)
  (bind _returnvalue (Animation|PlayAnimMontage "/Game/BP/CharacterBP/Anim/AM_Kick_Light_Montage.AM_Kick_Light_Montage" 1.0 "None"))
  (CallFunction|HaltMovement)
  (CallFunction|ComboUpdater)
  (Utilities|FlowControl|Delay _returnvalue)
  (CallFunction|UnlockAttack))

(event Custom|ComboTimerInit
  ;[0.15 0.15 0.15 0.5] Combo Managment
  (Utilities|Time|SetTimerbyEvent (delegate Custom|DecrementComboTimer) 1.0 true))

(event Custom|DecrementComboTimer
  ;[0.15 0.15 0.15 0.5] Combo Managment
  (if (<= (Variables|Default|GetComboTimer) 0.0)
    (Variables|Default|SetComboTimer 0.0)
    (else
      (Math|Float|DecrementFloat (Variables|Default|GetComboTimer)))))

(event Custom|OnAnimationEnd
  (params (AnimDelay :type Float%20%28double-precision%29))
  (Variables|Default|SetJabbing false)
  (Variables|Default|SetIsLightKicking? false)
  (Variables|Default|SetSmacking false)
  (Variables|Default|SetPerfectHeavy false)
  (Variables|Default|SetIsHeavyKicking? false)
  (Variables|Default|SetAttacking? false)
  (CallFunction|RestartMovement))

(event Custom|UnlockAttack
  ;[0.15 0.15 0.15 0.5] Stance Based Inputs
  (Utilities|FlowControl|Sequence
    (:then_0
      (Utilities|FlowControl|DoOnce false) ; enters at Reset
    )
    (:then_1
      (Utilities|FlowControl|DoOnce false) ; enters at Reset
    )))

(event Custom|RestartMovement
  ;[0.15 0.15 0.15 0.5] Basic Actions
  (Variables|/Script/Engine.CharacterMovementComponent|SetMaxWalkSpeed (Variables|Character|GetCharacterMovement) (Variables|Default|GetMovespeed)))

(event Custom|Take%20Damage
  (params (DamageRecieved :type Float%20%28double-precision%29))
  (if (Variables|Default|GetInvFrames)
    (CallFunction|Invincibility)
    (else
      (CallFunction|ReceiveDamage DamageRecieved)
      (Variables|Default|SetInvFrames true))))

(event Custom|Invincibility
  (Utilities|FlowControl|DelayUntilNextFrame)
  (Variables|Default|SetInvFrames false))

(event Custom|ComboUpdater
  (bind _combo_counter (Variables|Default|GetCombo%20Counter))
  ;[0.15 0.15 0.15 0.5] Combo Managment
  (if (Variables|Default|GetPerfectHeavy)
    (bind _output_get (Variables|Default|SetComboReader "PERFECT COMBO!"))
    (Rendering|Components|TextRender|SetText _combo_counter _output_get)
    (elif (== (Variables|Default|GetComboChecker) 1)
      (bind _output_get_2 (Variables|Default|SetComboReader "1x"))
      (Rendering|Components|TextRender|SetText _combo_counter _output_get_2)
      (elif (== (Variables|Default|GetComboChecker) 2)
        (bind _output_get_3 (Variables|Default|SetComboReader "2x"))
        (Rendering|Components|TextRender|SetText _combo_counter _output_get_3)
        (else
          (bind _output_get_4 (Variables|Default|SetComboReader ""))
          (Rendering|Components|TextRender|SetText _combo_counter _output_get_4)))))
  (if (<= (Variables|Default|GetComboTimer) 0.0)
    (bind _output_get_5 (Variables|Default|SetComboReader ""))
    (Rendering|Components|TextRender|SetText _combo_counter _output_get_5)
    (Variables|Default|SetComboChecker 0)))

(event Custom|Position%20ComboBox
  (bind _combo_counter (Variables|Default|GetCombo%20Counter))
  (bind _returnvalue (Transformation|GetWorldRotation _combo_counter))
  (Transformation|SetWorldRotation _combo_counter (Math|Rotator|MakeRotator (.roll _returnvalue) (.pitch _returnvalue) (- (.yaw (Transformation|GetWorldRotation (Variables|Character|GetMesh))) (.yaw _returnvalue))) false false))

(event Custom|Forfeit
  (Development|PrintString (Utilities|String|Append "Player " (Utilities|String|ToString(Integer) (Variables|Default|GetPlayerIndex)) "" "Has Conceided the match!") true true "(R=0.000000,G=0.660000,B=1.000000,A=1.000000)" 7.0)
  (Utilities|FlowControl|Delay 7.0))

(event Custom|HeavyAttack_Kick
  ;[0.15 0.15 0.15 0.5] Punching and Kicking
  (Variables|Default|SetIsHeavyKicking? true)
  (CallFunction|IncreaseComboTimer)
  (bind _returnvalue (Animation|PlayAnimMontage "/Game/BP/CharacterBP/Anim/AM_Kick_Heavy_Montage.AM_Kick_Heavy_Montage" 1.0 "None"))
  (CallFunction|HaltMovement)
  (CallFunction|ComboUpdater)
  (Utilities|FlowControl|Delay _returnvalue)
  (CallFunction|UnlockAttack))

(event Custom|HeavyAttack_Punch
  ;[0.15 0.15 0.15 0.5] Punching and Kicking
  (if (== (Variables|Default|GetComboChecker) 2)
    (Variables|Default|SetSmacking true)
    (Variables|Default|SetComboChecker 0)
    (Variables|Default|SetPerfectHeavy true)
    (CallFunction|IncreaseComboTimer)
    (else
      (Variables|Default|SetSmacking true)
      (Variables|Default|SetComboChecker 0)))
  (bind _returnvalue (Animation|PlayAnimMontage "/Game/BP/CharacterBP/Anim/AM_Attack_Heavy_Montage.AM_Attack_Heavy_Montage" 1.0 "None"))
  (CallFunction|HaltMovement)
  (CallFunction|ComboUpdater)
  (Utilities|FlowControl|Delay _returnvalue)
  (CallFunction|UnlockAttack))

(event Input|EnhancedActionEvents|EnhancedInputActionIA_OpenMenu
  (params (ActionValue :type Boolean) (ElapsedSeconds :type Float%20%28double-precision%29) (TriggeredSeconds :type Float%20%28double-precision%29) (InputAction :type Input%20Action%20Object%20Reference :default "/Game/BP/CharacterBP/InputActions/IA_OpenMenu.IA_OpenMenu"))
  (bind _myplayercontroller (Variables|Default|GetMyPlayerController))
  (:Started
    (Utilities|FlowControl|FlipFlop
      (:A
        (if (not (Variables|Default|GetIsPausemenuopen?))
          (Variables|Default|SetIsPausemenuopen? true)
          (bind _returnvalue (UserInterface|CreateWidget "/Game/BP/Menu/WBP_Options.WBP_Options_C" _myplayercontroller))
          (bind _output_get (Variables|Default|SetPauseMenu _returnvalue))
          (Variables|/Game/BP/Menu/WBP_Options.WBP_Options_C|SetIsPauseMenu? _output_get true)
          (Default|GetPlayerRef _output_get _myplayercontroller)
          (UserInterface|Viewport|AddtoViewport (Variables|Default|GetPauseMenu) 0)
          (Input|SetInputModeGameandUI _myplayercontroller (Variables|Default|GetPauseMenu) "DoNotLock" true false)
          (Game|SetGamePaused true)))
      (:B
        (Default|CloseUI (Variables|Default|GetPauseMenu))
        (Variables|Default|SetIsPausemenuopen? false)))))

(event Input|EnhancedActionEvents|EnhancedInputActionIA_Walk
  (params (ActionValue :type Float%20%28double-precision%29) (ElapsedSeconds :type Float%20%28double-precision%29) (TriggeredSeconds :type Float%20%28double-precision%29) (InputAction :type Input%20Action%20Object%20Reference :default "/Game/BP/CharacterBP/InputActions/IA_Walk.IA_Walk"))
  ;[0.15 0.15 0.15 0.5] Basic Actions
  (Pawn|Input|AddMovementInput (Math|Vector|GetForwardVector (Math|Rotator|MakeRotator 0.0 0.0 (.yaw (Pawn|GetControlRotation :!class /Script/Engine.Pawn)))) ActionValue false))

(event Input|EnhancedActionEvents|EnhancedInputActionIA_StanceChange
  (params (ActionValue :type Boolean) (ElapsedSeconds :type Float%20%28double-precision%29) (TriggeredSeconds :type Float%20%28double-precision%29) (InputAction :type Input%20Action%20Object%20Reference :default "/Game/BP/CharacterBP/InputActions/IA_StanceChange.IA_StanceChange"))
  ;[0.15 0.15 0.15 0.5] Stance Changing
  ;;[0.15 0.15 0.15 0.5] Checks that the stance you are changing to isnt dead.
  (:Started
    (Utilities|FlowControl|FlipFlop
      (:A
        (if (<= (Variables|Default|GetStance1HP) 0.0)
          (CallFunction|StanceFailed :!label _label)
          (else
            (Variables|Default|SetCurrentStance "NewEnumerator0")
            (CallFunction|UpdateStanceHPBar :!label _label_2))))
      (:B
        (if (<= (Variables|Default|GetStance2HP) 0.0)
          (goto _label)
          (else
            (Variables|Default|SetCurrentStance "NewEnumerator1")
            (goto _label_2)))))))

(event Input|EnhancedActionEvents|EnhancedInputActionIA_Crouch
  (params (ActionValue :type Boolean) (ElapsedSeconds :type Float%20%28double-precision%29) (TriggeredSeconds :type Float%20%28double-precision%29) (InputAction :type Input%20Action%20Object%20Reference :default "/Game/BP/CharacterBP/InputActions/IA_Crouch.IA_Crouch"))
  ;[0.15 0.15 0.15 0.5] Basic Actions
  (:Started
    (Variables|Default|SetCrouching true)
    (CallFunction|HaltMovement))
  (:Canceled
    (Variables|Default|SetCrouching false :!label _label)
    (CallFunction|RestartMovement))
  (:Completed
    (goto _label)))

(event Input|EnhancedActionEvents|EnhancedInputActionIA_LightAttack
  (params (ActionValue :type Boolean) (ElapsedSeconds :type Float%20%28double-precision%29) (TriggeredSeconds :type Float%20%28double-precision%29) (InputAction :type Input%20Action%20Object%20Reference :default "/Game/BP/CharacterBP/InputActions/IA_LightAttack.IA_LightAttack"))
  ;[0.15 0.15 0.15 0.5] Stance Based Inputs
  (:Started
    (Utilities|FlowControl|DoOnce false
      (:Completed
        (switch Utilities|FlowControl|Switch|SwitchonE_Stances (Variables|Default|GetCurrentStance)
          (:NewEnumerator0
            (CallFunction|LightAttackPunch))
          (:NewEnumerator1
            (CallFunction|LightAttackKick)))))))

(event Input|EnhancedActionEvents|EnhancedInputActionIA_HeavyAttack
  (params (ActionValue :type Boolean) (ElapsedSeconds :type Float%20%28double-precision%29) (TriggeredSeconds :type Float%20%28double-precision%29) (InputAction :type Input%20Action%20Object%20Reference :default "/Game/BP/CharacterBP/InputActions/IA_HeavyAttack.IA_HeavyAttack"))
  ;[0.15 0.15 0.15 0.5] Stance Based Inputs
  (:Started
    (Utilities|FlowControl|DoOnce false
      (:Completed
        (switch Utilities|FlowControl|Switch|SwitchonE_Stances (Variables|Default|GetCurrentStance)
          (:NewEnumerator0
            (CallFunction|HeavyAttackPunch))
          (:NewEnumerator1
            (CallFunction|HeavyAttackKick)))))))

(event Input|EnhancedActionEvents|EnhancedInputActionIA_ExplicitDodgeAction
  (params (ActionValue :type Boolean) (ElapsedSeconds :type Float%20%28double-precision%29) (TriggeredSeconds :type Float%20%28double-precision%29) (InputAction :type Input%20Action%20Object%20Reference :default "/Game/BP/CharacterBP/InputActions/IA_ExplicitDodgeAction.IA_ExplicitDodgeAction"))
  (bind _currentstance (Variables|Default|GetCurrentStance))
  ;[0.15 0.15 0.15 0.5] Stance Based Inputs
  (:Started
    (switch Utilities|FlowControl|Switch|SwitchonE_Stances _currentstance
      (:NewEnumerator0
        (Variables|Default|SetBlocking true)
        (CallFunction|HaltMovement)
        (Variables|Default|SetPerfectBlock? true)
        (Utilities|FlowControl|Delay 1.0)
        (Variables|Default|SetPerfectBlock? false))
      (:NewEnumerator1
        (Variables|Default|SetDashing true))))
  (:Canceled
    (switch Utilities|FlowControl|Switch|SwitchonE_Stances _currentstance :!label _label
      (:NewEnumerator0
        (Variables|Default|SetBlocking false)
        (CallFunction|RestartMovement))
      (:NewEnumerator1
        (Variables|Default|SetDashing false))))
  (:Completed
    (goto _label)))

(event EventBeginPlay
  ;[0.15 0.15 0.15 0.5] Round Start
  (Utilities|FlowControl|DelayUntilNextTick)
  (bind _asbp_player_controller (Utilities|Casting|CastToBP_PlayerController (Pawn|GetController)))
  (Utilities|IsValid (PlayerController|LocalPlayerSubsystems|GetEnhancedInputLocalPlayerSubsystem _asbp_player_controller)
    (:Is%20Valid
      (Input|AddMappingContext (PlayerController|LocalPlayerSubsystems|GetEnhancedInputLocalPlayerSubsystem _asbp_player_controller) "/Game/BP/CharacterBP/InputActions/InputMappingContext.InputMappingContext" 0 "(bIgnoreAllPressedKeysUntilRelease=True,bForceImmediately=False,bNotifyUserSettings=False)")
      (CallFunction|FindPlayerIndex)
      (CallFunction|SetHPtoMax)
      (bind _foundwidgets (Widget|GetAllWidgetsOfClass "/Game/BP/HUD/WBP_PlayerHUD.WBP_PlayerHUD_C" true))
      (Variables|Default|SetPlayerHUD (Utilities|Array|Get(acopy) _foundwidgets))
      (Variables|/Script/Engine.CharacterMovementComponent|SetMaxWalkSpeed (Variables|Character|GetCharacterMovement) (Variables|Default|GetMovespeed))
      (CallFunction|PositionComboBox)
      (CallFunction|ComboTimerInit)
      (bind _asgi_fighting_instance (Utilities|Casting|CastToGI_FightingInstance (Game|GetGameInstance)))
      (Default|RoundStart _asgi_fighting_instance (Variables|/Game/BP/CharacterBP/GI_FightingInstance.GI_FightingInstance_C|GetRoundNumber _asgi_fighting_instance)))))

(fn ConstructionScript)

(fn SetHPtoMax
  (bind _stance1hp_max (Variables|Default|GetStance1HP_Max))
  (bind _stance2hp_max (Variables|Default|GetStance2HP_Max))
  (Variables|Default|SetStance1HP _stance1hp_max)
  (Variables|Default|SetStance2HP _stance2hp_max)
  (bind _output_get (Variables|Default|SetOverallHP_Max (+ _stance1hp_max _stance2hp_max)))
  (Variables|Default|SetOverallHP _output_get))

(fn UpdateHealth
  (bind _playerhud (Variables|Default|GetPlayerHUD))
  (Variables|Default|SetOverallHP (+ (Variables|Default|GetStance1HP) (Variables|Default|GetStance2HP)))
  (Utilities|FlowControl|Sequence
    (:then_0
      (Default|UpdateP1Health _playerhud))
    (:then_1
      (Default|UpdateP2Health _playerhud))))

(fn ReceiveDamage
  (params (Damage%20Recieved :type Float%20%28double-precision%29))
  (if (and (<= (Variables|Default|GetStance1HP) 0.0) (<= (Variables|Default|GetStance2HP) 0.0))
    (bind _asgi_fighting_instance (Utilities|Casting|CastToGI_FightingInstance (Game|GetGameInstance)))
    (Default|RoundOver _asgi_fighting_instance (Variables|Default|GetPlayerIndex))
    (else
      (switch Utilities|FlowControl|Switch|SwitchonE_Stances (Variables|Default|GetCurrentStance)
        (:NewEnumerator0
          (if (Variables|Default|GetBlocking)
            (if (Variables|Default|GetPerfectBlock?)
              (bind _output_get (Variables|Default|SetStance1HP (- (Variables|Default|GetStance1HP) (- Damage%20Recieved (/ Damage%20Recieved 1.25)))))
              (if (<= _output_get 0.0)
                (Variables|Default|SetCurrentStance "NewEnumerator1")
                (CallFunction|ReceiveDamage (* _output_get -1.0))
                (Components|DestroyComponent (Variables|Default|GetCable4) :!label _label)
                (CallFunction|UpdateStanceHPBar :!label _label_2)
                (else
                  (CallFunction|UpdateHealth :!label _label_3)))
              (else
                (bind _output_get_2 (Variables|Default|SetStance1HP (- (Variables|Default|GetStance1HP) (- Damage%20Recieved (/ Damage%20Recieved 2.0)))))
                (if (<= _output_get_2 0.0)
                  (Variables|Default|SetCurrentStance "NewEnumerator1")
                  (CallFunction|ReceiveDamage (* _output_get_2 -1.0))
                  (goto _label)
                  (else
                    (goto _label_3)))))
            (else
              (bind _output_get_3 (Variables|Default|SetStance1HP (- (Variables|Default|GetStance1HP) Damage%20Recieved)))
              (if (<= _output_get_3 0.0)
                (Variables|Default|SetCurrentStance "NewEnumerator1")
                (CallFunction|ReceiveDamage (* _output_get_3 -1.0))
                (goto _label)
                (else
                  (goto _label_3))))))
        (:NewEnumerator1
          (bind _output_get_4 (Variables|Default|SetStance2HP (- (Variables|Default|GetStance2HP) Damage%20Recieved)))
          (if (<= _output_get_4 0.0)
            (Variables|Default|SetCurrentStance "NewEnumerator0")
            (CallFunction|ReceiveDamage (* _output_get_4 -1.0))
            (Components|DestroyComponent (Variables|Default|GetCable1))
            (goto _label_2)
            (else
              (goto _label_3))))))))

(fn UpdateStanceHPBar
  (bind _playerhud (Variables|Default|GetPlayerHUD))
  (bind _playerhud_2 (Variables|Default|GetPlayerHUD))
  (bind _widgetswitcher_p2 (Variables|/Game/BP/HUD/WBP_PlayerHUD.WBP_PlayerHUD_C|GetWidgetSwitcher_P2 _playerhud))
  (bind _widgetswitcher_p1 (Variables|/Game/BP/HUD/WBP_PlayerHUD.WBP_PlayerHUD_C|GetWidgetSwitcher_P1 _playerhud_2))
  (if (== (Variables|Default|GetPlayerIndex) 0)
    (switch Utilities|FlowControl|Switch|SwitchonE_Stances (Variables|Default|GetCurrentStance)
      (:NewEnumerator0
        (Class|WidgetSwitcher|SetActiveWidget _widgetswitcher_p1 (Variables|/Game/BP/HUD/WBP_PlayerHUD.WBP_PlayerHUD_C|GetP1Stance1HealthBar _playerhud_2)))
      (:NewEnumerator1
        (Class|WidgetSwitcher|SetActiveWidget _widgetswitcher_p1 (Variables|/Game/BP/HUD/WBP_PlayerHUD.WBP_PlayerHUD_C|GetP1Stance2HealthBar _playerhud_2))))
    (else
      (switch Utilities|FlowControl|Switch|SwitchonE_Stances (Variables|Default|GetCurrentStance)
        (:NewEnumerator0
          (Class|WidgetSwitcher|SetActiveWidget _widgetswitcher_p2 (Variables|/Game/BP/HUD/WBP_PlayerHUD.WBP_PlayerHUD_C|GetP2Stance1HealthBar _playerhud)))
        (:NewEnumerator1
          (Class|WidgetSwitcher|SetActiveWidget _widgetswitcher_p2 (Variables|/Game/BP/HUD/WBP_PlayerHUD.WBP_PlayerHUD_C|GetP2Stance2HealthBar _playerhud)))))))

(fn FindPlayerIndex
  (bind _returnvalue (Game|GetGameMode))
  (bind _asbp_main_game_mode (Utilities|Casting|CastToBP_MainGameMode _returnvalue))
  (Variables|Default|SetPlayer%201 (Variables|/Game/BP/CharacterBP/BP_MainGameMode.BP_MainGameMode_C|GetPlayer1 _asbp_main_game_mode))
  (Variables|Default|SetPlayer%202 (Variables|/Game/BP/CharacterBP/BP_MainGameMode.BP_MainGameMode_C|GetPlayer2 _asbp_main_game_mode))
  (bind _outactors (Actor|GetAllActorsOfClass "/Game/BP/CharacterBP/BP_PlayerController.BP_PlayerController_C"))
  (if (== (Pawn|GetController self) (Utilities|Array|Get(acopy) _outactors))
    (Variables|Default|SetMyPlayerController (Variables|Default|GetPlayer%201))
    (Variables|Default|SetPlayerIndex 0)
    (Development|PrintString "I am player 1" true true "(R=1.000000,G=0.075250,B=0.000000,A=1.000000)")
    (else
      (Variables|Default|SetMyPlayerController (Variables|Default|GetPlayer%202))
      (Variables|Default|SetPlayerIndex 1)
      (Development|PrintString "I am player 2" true true "(R=0.295078,G=1.000000,B=0.000000,A=1.000000)"))))

(fn GetPlayerStats)