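; Game mode that sets up local multiplayer and hands out spawn points to players.
; On BeginPlay it creates a player on controller ID 1 with its own player controller.
; The construction script caches all PlayerStart actors, and the ChoosePlayerStart override returns the first cached entry and removes it, so successive players get different starts.
; The list is consumed in retrieval order, with no refill or empty check.
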(event EventBeginPlay
  (Class|GameplayStatics|CreatePlayer 1))

(fn ConstructionScript
  (bind _outactors (Actor|GetAllActorsOfClass "/Script/Engine.PlayerStart"))
  (Variables|Default|SetPlayerSpawns _outactors))

(fn ChoosePlayerStart
  (params (Player :type Controller%20Object%20Reference))
  (bind _playerspawns (Variables|Default|GetPlayerSpawns))
  (bind _output_get (Variables|Default|SetSelectedSpawn (Utilities|Array|Get(acopy) _playerspawns)))
  (Utilities|Array|RemoveItem _playerspawns _output_get)
  (return (Variables|Default|GetSelectedSpawn)))